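; Base interactable Blueprint that shows a text prompt while the player is nearby, leaving Interact as an empty function.
; Overlap events on its Box toggle TextRender visibility for BP_Player, and the text starts hidden.
; On BeginPlay, it sets ChildActor's relative rotation once using a look-at toward a CameraActor, calculated from that component's rotation X vector rather than its location.
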(event `self.ReceiveBeginPlay`
  (`self.ToggleUI` false)
  (bind _returnvalue (`GameplayStatics.GetActorOfClass` "/Script/Engine.CameraActor"))
  (bind _returnvalue_location (`KismetMathLibrary.BreakTransform` (`self.GetTransform` _returnvalue)))
  (`SceneComponent.K2_SetRelativeRotation` (`self.ChildActor`) (`KismetMathLibrary.FindLookAtRotation` (`KismetMathLibrary.Conv_RotatorToVector` (`SceneComponent.RelativeRotation` (`self.ChildActor`))) _returnvalue_location) false false))

(event `self.Box.OnComponentBeginOverlap`
  (params (OverlappedComponent :type "PrimitiveComponent Object Reference") (OtherActor :type "Actor Object Reference") (OtherComp :type "PrimitiveComponent Object Reference") (OtherBodyIndex :type Integer) (bFromSweep :type Boolean) (SweepResult :type "HitResult Structure (by ref)"))
  (cast `/Game/Objects/Player/Blueprints/BP_Player` OtherActor)
  (`self.ToggleUI` true))

(event `self.Box.OnComponentEndOverlap`
  (params (OverlappedComponent :type "PrimitiveComponent Object Reference") (OtherActor :type "Actor Object Reference") (OtherComp :type "PrimitiveComponent Object Reference") (OtherBodyIndex :type Integer))
  (cast `/Game/Objects/Player/Blueprints/BP_Player` OtherActor)
  (`self.ToggleUI` false))

(fn `Interact`)

(fn `ToggleUI`
  (params (bNewVisibility :type Boolean))
  (`SceneComponent.SetVisibility` (`self.TextRender`) bNewVisibility false))

(fn `UserConstructionScript`)