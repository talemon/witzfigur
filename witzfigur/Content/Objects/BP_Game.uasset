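; BP_Game runs a card game built on Attention, Confusion and Laughter stats, special tokens and limited action points.
; It creates the WB_Card UI and binds its success and failure events, which both apply clamped stat effects, update tokens and spend an action point.
; Only success adds a random score within the card's range.
; Each play rechecks card requirements, and exhausted points swap in WBP_ScoreScreen with the final score.
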(event `self.ReceiveBeginPlay`
  (bind _returnvalue (`|CreateWidget` "/Game/Objects/Widgets/WB_Card.WB_Card_C"))
  (`UserWidget.AddToViewport` _returnvalue 0)
  (add `/Game/Objects/Widgets/WB_Card.CardSuccess` _returnvalue (`|CreateDelegate` :!event `onSuccess`))
  (set `self.UIGAME` _returnvalue)
  (add `/Game/Objects/Widgets/WB_Card.CardFailed` _returnvalue (`|CreateDelegate` :!event `OnFailed`))
  (`self.CheckCardsPlayable`))

(event `onSuccess`
  (params (Data :type "/Game/Data/Structs/STR_RangeOfEffects Structure"))
  (bind (_min _max) (break `/Game/Data/Structs/STR_FromMinToMax` (`.Score_10_BA4349E94FCFF661CF2EFDA731F9930B` (break `/Game/Data/Structs/STR_RangeOfEffects` Data))))
  (`self.AddTokens` Data)
  (`self.SetNiceInts` Data)
  (set `self.Score` (+ (`self.Score`) (`KismetMathLibrary.RandomIntegerInRange` (`KismetMathLibrary.FTrunc` _min) (`KismetMathLibrary.FTrunc` _max))))
  (bind _result (`/Engine/EditorBlueprintResources/StandardMacros.DecrementInt` (`self.ActionPoints`) :!label _label)
    (:`  `
      (`self.CheckCardsPlayable`)
      (if (<= _result 0)
        (bind _returnvalue (`|CreateWidget` "/Game/Level/Widgets/WBP_ScoreScreen.WBP_ScoreScreen_C"))
        (`UserWidget.AddToViewport` _returnvalue 0)
        (`/Game/Level/Widgets/WBP_ScoreScreen.SetScore` _returnvalue (`KismetStringLibrary.Conv_IntToString` (`self.Score`)))
        (`Widget.RemoveFromParent` (`self.UIGAME`))))))

(event `OnFailed`
  (params (Data :type "/Game/Data/Structs/STR_RangeOfEffects Structure"))
  (`self.AddTokens` Data)
  (`self.SetNiceInts` Data)
  (goto _label))

(fn `AddTokens`
  (params (STR_RangeOfEffects :type "/Game/Data/Structs/STR_RangeOfEffects Structure (by ref)"))
  (locals (value :type Integer))
  (bind (_attention _confusion _laughter _special) (break `/Game/Data/Structs/STR_RangeOfEffects` STR_RangeOfEffects))
  (bind _specialtokens (`self.SpecialTokens`))
  (if (not (`|EnumEquality` _special "NewEnumerator5"))
    (bind _output_get (set `local.value` (`BlueprintMapLibrary.Map_Find` _specialtokens _special)))
    (`/Engine/EditorBlueprintResources/StandardMacros.IncrementInt` _output_get
      (:`  `
        (`BlueprintMapLibrary.Map_Add` _specialtokens _special)))))

(fn `CheckCardsPlayable`
  (for _array_element (`/Game/Objects/Widgets/WB_Card.BetterButtons` (`self.UIGAME`))
    (bind _data (`/Game/Objects/Widgets/WBP_Button.Data` _array_element))
    (`/Game/Objects/Widgets/WBP_Button.SetPlayable` _array_element (and (== (>= (`self.attention`) (break `/Game/Data/Structs/STR_Requirements` (`.Requirements_7_EF767FE840070984BFCB0FB03172DE28` (break `/Game/Data/Structs/STR_CardData` _data)))) true) (== (<= (`self.Confusion`) (`.Confusion_9_D90820AB4D83E3538C3BA0A3CF26459E` (break `/Game/Data/Structs/STR_Requirements` (`.Requirements_7_EF767FE840070984BFCB0FB03172DE28` (break `/Game/Data/Structs/STR_CardData` _data))))) true) (== (>= (`self.Laughter`) (`.laughter_10_1A550E1245544212148CF6AB4AC0FB03` (break `/Game/Data/Structs/STR_Requirements` (`.Requirements_7_EF767FE840070984BFCB0FB03172DE28` (break `/Game/Data/Structs/STR_CardData` _data))))) true) (or (== (`|EnumEquality` (`.Special_11_3155CA434EB4070832A714AA0402C011` (break `/Game/Data/Structs/STR_Requirements` (`.Requirements_7_EF767FE840070984BFCB0FB03172DE28` (break `/Game/Data/Structs/STR_CardData` _data)))) "NewEnumerator5") true) (== (>= (`BlueprintMapLibrary.Map_Find` (`self.SpecialTokens`) (`.Special_11_3155CA434EB4070832A714AA0402C011` (break `/Game/Data/Structs/STR_Requirements` (`.Requirements_7_EF767FE840070984BFCB0FB03172DE28` (break `/Game/Data/Structs/STR_CardData` _data))))) 1) true))))
    (`/Game/Objects/Widgets/WB_Card.UpdateValues` (`self.UIGAME`) (`self.Confusion`) (`self.Laughter`) (`self.attention`) (`self.ActionPoints`))))

(fn `EnoughTokens`
  (returns (result :type Boolean))
  (return (<= (`self.ActionPoints`) 0)))

(fn `SetNiceInts`
  (params (STR_RangeOfEffects :type "/Game/Data/Structs/STR_RangeOfEffects Structure (by ref)"))
  (bind (_attention _confusion _laughter) (break `/Game/Data/Structs/STR_RangeOfEffects` STR_RangeOfEffects))
  (set `self.attention` (`KismetMathLibrary.Clamp` (+ (`self.attention`) _attention) 0 100))
  (set `self.Confusion` (`KismetMathLibrary.Clamp` (+ _confusion (`self.Confusion`)) 0 100))
  (set `self.Laughter` (`KismetMathLibrary.Clamp` (+ _laughter (`self.Laughter`)) 0 100)))

(fn `UserConstructionScript`)