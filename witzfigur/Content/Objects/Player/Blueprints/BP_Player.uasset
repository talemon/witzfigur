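; BP_Player is the player pawn, handling movement and interaction through Enhanced Input.
; On BeginPlay it adds the IMC_Player mapping context to player 0.
; IA_Move feeds movement input along the capsule's right and forward vectors.
; IA_Interact calls Interact on the first BP_BaseInteractable overlapping the capsule, leaving the response to that actor.
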(event `self.ReceiveBeginPlay`
  (`EnhancedInputSubsystemInterface.AddMappingContext` (pcsubsystem `EnhancedInputLocalPlayerSubsystem` (`GameplayStatics.GetPlayerController` 0)) "/Game/Input/IMC_Player.IMC_Player" 0 (struct)))

(event `EnhancedInput|/Game/Input/InputActions/IA_Move`
  (params (ActionValue :type "Vector2D Structure") (ElapsedSeconds :type "Float (double-precision)") (TriggeredSeconds :type "Float (double-precision)") (InputAction :type "InputAction Object Reference" :default "/Game/Input/InputActions/IA_Move.IA_Move"))
  (bind (_x _y) (`KismetMathLibrary.BreakVector2D` ActionValue))
  (:`Triggered`
    (`self.AddMovementInput` (`SceneComponent.GetRightVector` (`self.CapsuleComponent`)) _x)
    (`self.AddMovementInput` (`SceneComponent.GetForwardVector` (`self.CapsuleComponent`)) _y)))

(event `EnhancedInput|/Game/Input/InputActions/IA_Interact`
  (params (ActionValue :type Boolean) (ElapsedSeconds :type "Float (double-precision)") (TriggeredSeconds :type "Float (double-precision)") (InputAction :type "InputAction Object Reference" :default "/Game/Input/InputActions/IA_Interact.IA_Interact"))
  (bind _output (`|GetArrayItem` (`PrimitiveComponent.GetOverlappingActors` (`self.CapsuleComponent`) "/Game/Objects/Interactable/BP_BaseInteractable.BP_BaseInteractable_C")))
  (:`Triggered`
    (`/Engine/EditorBlueprintResources/StandardMacros.IsValid` _output
      (:`Is Valid`
        (bind _asbp_base_interactable (cast `/Game/Objects/Interactable/BP_BaseInteractable` _output))
        (`/Game/Objects/Interactable/BP_BaseInteractable.Interact` _asbp_base_interactable)))))

(fn `UserConstructionScript`)